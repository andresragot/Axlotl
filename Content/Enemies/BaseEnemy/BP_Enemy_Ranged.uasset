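; Ranged enemy character, with an attack, a health bar and destruction when damage drains its health.
; Attack plays a montage and immediately traces from Lanzador to the AI controller's AttackTarget, applying instant damage if nothing blocks the trace.
; Montage completion or interruption calls AttackEnd.
; Tick refreshes the health widget assuming 100 maximum health, while functions set walk speed by movement state and report ideal attack and defend radii.
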(event EventBeginPlay)

(event Collision|EventActorBeginOverlap
  (params (OtherActor :type Actor%20Object%20Reference)))

(event EventTick
  (params (DeltaSeconds :type Float%20%28single-precision%29))
  ;[1 0.9288 0.2916] Event tick
  (bind _aswb_ranged_enemy (Utilities|Casting|CastToWB_RangedEnemy (UserInterface|GetWidget (Variables|Default|GetHealthBar))))
  (Progress|SetPercent (Variables|/Game/Widgets/Enemies/WB_RangedEnemy.WB_RangedEnemy_C|GetHealthBar _aswb_ranged_enemy) (/ (Variables|Default|GetEnemy_Health) 1e+02)))

(event EventAttack
  ;[1 0 0.8928] Ataque
  ;;[1 1 1] Animacion de Ataque rango
  (Animation|Montage|PlayMontage (Variables|Character|GetMesh) "/Game/Player/Animations/AttackMontage.AttackMontage"
    (:then
      (bind _asaicontroller_base_enemy (Utilities|Casting|CastToAIController_BaseEnemy (AI|GetAIController self)))
      (bind _attack_target (Variables|/Game/Enemies/BaseEnemy/AI/AIController_BaseEnemy.AIController_BaseEnemy_C|GetAttack%20Target _asaicontroller_base_enemy)
        (:then
          (bind _returnvalue (Collision|LineTraceByChannel (Transformation|GetWorldLocation (Variables|Default|GetLanzador)) (Transformation|GetActorLocation _attack_target) "TraceTypeQuery1" false 0 "ForDuration"))
          (if (not _returnvalue)
            (Development|PrintString "Hit target")
            (Game|Damage|ApplyDamage _attack_target (Variables|Default|GetEnemy_Dmg) 0 0)))
        (:else)))
    (:OnCompleted
      (Default|CallAttackEnd :!label _label))
    (:OnInterrupted
      (goto _label))))

(event Game|Damage|EventAnyDamage
  (params (Damage :type Float%20%28single-precision%29) (DamageType :type Damage%20Type%20Object%20Reference) (InstigatedBy :type Controller%20Object%20Reference) (DamageCauser :type Actor%20Object%20Reference))
  ;[1 0.01553 0] Recibir daño
  (bind _output_get (Variables|Default|SetEnemy_Health (- (Variables|Default|GetEnemy_Health) Damage)))
  (if (<= _output_get 0.0)
    (Actor|DestroyActor)))

(fn ConstructionScript
  (|CallParentFunction))

(fn SetMovementSpeed
  (params (Speed :type E_MovementSpeed%20Enum :default "NewEnumerator0"))
  (bind _output_get (Variables|/Script/Engine.CharacterMovementComponent|SetMaxWalkSpeed (Variables|Character|GetCharacterMovement) (Utilities|Select :Index Speed :NewEnumerator0 0.0 :NewEnumerator1 2e+02 :NewEnumerator3 3e+02 :NewEnumerator2 5e+02)))
  (return _output_get))

(fn GetIdealRange
  (return 6e+02 6e+02))