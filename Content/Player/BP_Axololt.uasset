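; Player character for the axolotl, handling combat, dash, pausing, interaction and health UI.
; The saved weapon choice selects Ranged or Light, switching attack inputs between spawned projectiles and timed attack flags, with hard attacks briefly locking movement and dash.
; Tick refreshes the health bar and levels ranged projectile pitch.
; Death shows a death widget and saves reset health, room and weapon stats, while Interact messages overlapping Interactable actors.
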(event Input|EnhancedActionEvents|EnhancedInputActionPauseGame
  (params (ActionValue :type Boolean) (ElapsedSeconds :type Float%20%28double-precision%29) (TriggeredSeconds :type Float%20%28double-precision%29) (InputAction :type Input%20Action%20Object%20Reference :default "/Game/Player/Input/Actions/PauseGame.PauseGame"))
  (bind _returnvalue (Game|GetPlayerController 0))
  ;[1 1 1] Pausar juego
  (:Started
    (if (not (Variables|Default|GetPauseMenu))
      (Variables|Default|SetPauseMenu true)
      (bind _returnvalue_2 (UserInterface|CreateWidget "/Game/Widgets/Menu/WB_PauseMenu.WB_PauseMenu_C" _returnvalue))
      (bind _output_get (Variables|Default|SetPauseMenuWidget _returnvalue_2))
      (UserInterface|Viewport|AddtoViewport _output_get 0)
      (Input|SetInputModeGameandUI _returnvalue (Variables|Default|GetPauseMenuWidget) "DoNotLock" true false)
      (Variables|/Script/Engine.PlayerController|SetbShowMouseCursor (Game|GetPlayerController 0) true)
      (Game|SetGamePaused true)
      (else
        (Variables|Default|SetPauseMenu false)
        (Widget|RemovefromParent (Variables|Default|GetPauseMenuWidget))
        (Game|SetGamePaused false)
        (Input|SetInputModeGameOnly _returnvalue false)
        (Variables|/Script/Engine.PlayerController|SetbShowMouseCursor (Game|GetPlayerController 0) false)))))

(event Input|EnhancedActionEvents|EnhancedInputActionInteractuar
  (params (ActionValue :type Boolean) (ElapsedSeconds :type Float%20%28double-precision%29) (TriggeredSeconds :type Float%20%28double-precision%29) (InputAction :type Input%20Action%20Object%20Reference :default "/Game/Player/Input/Actions/Interactuar.Interactuar"))
  ;[0.3996 1 0.4393] Interactuar
  (bind _array_element (Utilities|Array|ForEachLoopwithBreak (Collision|GetOverlappingActors "/Script/Engine.Actor" :!class /Script/Engine.Actor))
    (:LoopBody
      (if (Utilities|DoesObjectImplementInterface _array_element "/Game/Interface/Interactable.Interactable_C")
        (Class|Interactable|Interactable(Message) _array_element)))))

(event Input|EnhancedActionEvents|EnhancedInputActionLAttackAction
  (params (ActionValue :type Boolean) (ElapsedSeconds :type Float%20%28double-precision%29) (TriggeredSeconds :type Float%20%28double-precision%29) (InputAction :type Input%20Action%20Object%20Reference :default "/Game/Player/Input/Actions/LAttackAction.LAttackAction"))
  ;[1 0.4502 0.9048] Light Attack
  (switch Utilities|FlowControl|Switch|SwitchonEnum_Weapons (Variables|Default|GetEnum_weapons)
    (:NewEnumerator0
      (Game|SpawnActorfromClass "/Game/FirstPerson/Blueprints/BP_FirstPersonProjectile.BP_FirstPersonProjectile_C" (Transformation|GetWorldTransform (Variables|Default|GetSpawn%20Transform)) "Undefined" "MultiplyWithRoot" 0 self))
    (:NewEnumerator1
      (Variables|Default|SetAtaque_Basico true)
      (Utilities|FlowControl|Delay 0.5)
      (Variables|Default|SetAtaque_Basico false))))

(event Input|EnhancedActionEvents|EnhancedInputActionMoveAction
  (params (ActionValue :type Vector%202D%20Structure) (ElapsedSeconds :type Float%20%28double-precision%29) (TriggeredSeconds :type Float%20%28double-precision%29) (InputAction :type Input%20Action%20Object%20Reference :default "/Game/Player/Input/Actions/MoveAction.MoveAction"))
  ;[0.2778 0.6936 1] Move
  (:Triggered
    (Variables|Default|SetMoving true))
  (:Ongoing
    (Variables|Default|SetMoving true))
  (:Canceled
    (Variables|Default|SetMoving false :!label _label))
  (:Completed
    (goto _label)))

(event Input|EnhancedActionEvents|EnhancedInputActionHAttackAction
  (params (ActionValue :type Boolean) (ElapsedSeconds :type Float%20%28double-precision%29) (TriggeredSeconds :type Float%20%28double-precision%29) (InputAction :type Input%20Action%20Object%20Reference :default "/Game/Player/Input/Actions/HAttackAction.HAttackAction"))
  ;[1 0.01578 0.8583] Hard Attack
  (switch Utilities|FlowControl|Switch|SwitchonEnum_Weapons (Variables|Default|GetEnum_weapons)
    (:NewEnumerator0
      (Game|SpawnActorfromClass "/Game/Player/Actors/BP_Axo_Projectile_2.BP_Axo_Projectile_2_C" (Transformation|GetWorldTransform (Variables|Default|GetSpawn%20Transform)) "Undefined" "MultiplyWithRoot" 0 self)
      (Variables|Default|SetDash_Disable true)
      (Variables|/Script/Engine.MovementComponent|SetVelocity (Variables|Character|GetCharacterMovement) "0, 0, 0")
      (Input|SetIgnoreMoveInput (Game|GetPlayerController 0) true)
      (Utilities|FlowControl|Delay 0.3)
      (Input|SetIgnoreMoveInput (Game|GetPlayerController 0) false)
      (Variables|Default|SetDash_Disable false))
    (:NewEnumerator1
      (Variables|Default|SetAtaque_Especial true)
      (Variables|Default|SetDash_Disable true)
      (Variables|/Script/Engine.MovementComponent|SetVelocity (Variables|Character|GetCharacterMovement) "0, 0, 0")
      (Input|SetIgnoreMoveInput (Game|GetPlayerController 0) true)
      (Utilities|FlowControl|Delay 0.7)
      (Variables|Default|SetAtaque_Especial false)
      (Variables|Default|SetDash_Disable false)
      (Input|SetIgnoreMoveInput (Game|GetPlayerController 0) false))))

(event Input|EnhancedActionEvents|EnhancedInputActionDashAction
  (params (ActionValue :type Boolean) (ElapsedSeconds :type Float%20%28double-precision%29) (TriggeredSeconds :type Float%20%28double-precision%29) (InputAction :type Input%20Action%20Object%20Reference :default "/Game/Player/Input/Actions/DashAction.DashAction"))
  (bind _sp_dash_vfx (Variables|Default|GetSP_Dash_VFX))
  ;[0.5367 1 0.2852] Dash
  (if (not (Variables|Default|GetDash_Disable))
    (Variables|Default|SetDash ActionValue)
    (if (Variables|Default|GetMoving)
      (Rendering|SetVisibility (Variables|Character|GetMesh) false false)
      (Niagara|SpawnSystemAttached "/Game/VFX/NS_Dash.NS_Dash" _sp_dash_vfx "None" (Transformation|GetWorldLocation _sp_dash_vfx) (Math|Rotator|MakeRotator 0.0 0.0 (.yaw (Math|Conversions|RotationFromXVector (Transformation|GetActorForwardVector)))) "KeepWorldPosition" true)
      (Utilities|FlowControl|Delay 0.4)
      (Rendering|SetVisibility (Variables|Character|GetMesh) true false))
    (Variables|Default|SetDash false)))

(event EventBeginPlay
  ;[0.8334 1 0.03794] BeginPlay
  (CallFunction|LoadGame (Variables|Default|GetSlotNameSave))
  (if (== (Variables|Default|GetWeaponSelected) 0.0)
    (Variables|Default|SetEnum_weapons "NewEnumerator0")
    (else
      (Variables|Default|SetEnum_weapons "NewEnumerator1")))
  (bind _returnvalue (UserInterface|CreateWidget "/Game/Widgets/Player/WB_Player.WB_Player_C"))
  (bind _output_get (Variables|Default|SetUI_HealthBar _returnvalue))
  (UserInterface|Viewport|AddtoViewport _output_get 0))

(event EventTick
  (params (DeltaSeconds :type Float%20%28single-precision%29))
  ;[0.9134 1 0.3744] Event tick
  (Default|UpdateHealth (Variables|Default|GetUI_HealthBar) (Variables|Default|GetHealth))
  (switch Utilities|FlowControl|Switch|SwitchonEnum_Weapons (Variables|Default|GetEnum_weapons)
    (:NewEnumerator0
      (Class|Axololt|RangedAttack)
      (bind _output_get (Variables|Default|SetRotatorProjectile (Math|Rotator|MakeRotator (.roll (Variables|Default|GetRotatorProjectile)) 0.0 (.yaw (Variables|Default|GetRotatorProjectile)))))
      (Transformation|SetRelativeRotation (Variables|Default|GetSpawn%20Transform) _output_get false false))))

(event Game|Damage|EventAnyDamage
  (params (Damage :type Float%20%28single-precision%29) (DamageType :type Damage%20Type%20Object%20Reference) (InstigatedBy :type Controller%20Object%20Reference) (DamageCauser :type Actor%20Object%20Reference))
  ;[1 0 0.04479] Apply damage
  (Variables|Default|SetHealth (- (Variables|Default|GetHealth) Damage))
  (bind _output_get (Variables|Default|SetGet_Health (<= (Variables|Default|GetHealth) 0.0)))
  (if _output_get
    (Actor|DestroyActor)
    (bind _returnvalue (UserInterface|CreateWidget "/Game/Widgets/Menu/WB_Death.WB_Death_C"))
    (UserInterface|Viewport|AddtoViewport _returnvalue 0)
    (Variables|/Script/Engine.PlayerController|SetbShowMouseCursor (Game|GetPlayerController 0) true)
    (Variables|Default|SetHealth 1e+02)
    (Variables|Default|SetRoomCounter 0.0)
    (Variables|Default|SetWeaponSelected 0.0)
    (CallFunction|SaveGame (Variables|Default|GetSlotNameSave))))

(fn ConstructionScript)

(fn SaveGame
  (params (Slot%20Name :type String))
  (bind _returnvalue (SaveGame|DoesSaveGameExist Slot%20Name))
  (if _returnvalue
    (bind _returnvalue_2 (SaveGame|LoadGamefromSlot Slot%20Name))
    (Variables|Default|SetSave_REF _returnvalue_2)
    (else
      (bind _returnvalue_3 (SaveGame|CreateSaveGameObject "/Game/Instances/SaveStats.SaveStats_C"))
      (bind _output_get (Variables|Default|SetSave_REF _returnvalue_3))))
  (bind _assave_stats (Utilities|Casting|CastToSaveStats _output_get))
  (Variables|/Game/Instances/SaveStats.SaveStats_C|SetHealth _assave_stats (Variables|Default|GetHealth))
  (Variables|/Game/Instances/SaveStats.SaveStats_C|SetRoomCounter _assave_stats (Variables|Default|GetRoomCounter))
  (Variables|/Game/Instances/SaveStats.SaveStats_C|SetWeaponSelected _assave_stats (Variables|Default|GetWeaponSelected))
  (SaveGame|SaveGametoSlot (Variables|Default|GetSave_REF) Slot%20Name))

(fn LoadGame
  (params (Slot%20Name :type String))
  (bind _returnvalue (SaveGame|DoesSaveGameExist Slot%20Name))
  (if _returnvalue
    (bind _returnvalue_2 (SaveGame|LoadGamefromSlot Slot%20Name))
    (bind _assave_stats (Utilities|Casting|CastToSaveStats _returnvalue_2))
    (Variables|Default|SetHealth (Variables|/Game/Instances/SaveStats.SaveStats_C|GetHealth _assave_stats))
    (Variables|Default|SetWeaponSelected (Variables|/Game/Instances/SaveStats.SaveStats_C|GetWeaponSelected _assave_stats))
    (Variables|Default|SetRoomCounter (Variables|/Game/Instances/SaveStats.SaveStats_C|GetRoomCounter _assave_stats))
    (Variables|Default|SetRoomNumber (Variables|/Game/Instances/SaveStats.SaveStats_C|GetRoomNumber _assave_stats))))