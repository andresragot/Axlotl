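; BP_RoomChange is a trigger actor that handles room transitions for the BP_Axololt player.
; On overlap it increments and saves the player's RoomCounter, plays a shutter sound and fade widget, then after a delay opens the Boss level on the tenth room.
; Otherwise it re-rolls a random room until it differs from RoomNumber, but only prints it.
; The switch that would open that room's level is disconnected.
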(event OnComponentBeginOverlap(Trigger)
  (params (OverlappedComponent :type Primitive%20Component%20Object%20Reference) (OtherActor :type Actor%20Object%20Reference) (OtherComp :type Primitive%20Component%20Object%20Reference) (OtherBodyIndex :type Integer) (bFromSweep :type Boolean) (SweepResult :type Hit%20Result%20Structure%20%28by%20ref%29))
  (bind _asbp_axololt (Utilities|Casting|CastToBP_Axololt OtherActor))
  (bind _output_get (Variables|/Game/Player/BP_Axololt.BP_Axololt_C|SetRoomCounter _asbp_axololt (+ (Variables|/Game/Player/BP_Axololt.BP_Axololt_C|GetRoomCounter _asbp_axololt) 1.0)))
  (Default|SaveGame _asbp_axololt (Variables|Default|GetSlot%20Name%20Save))
  (Audio|PlaySound2D "/Engine/VREditor/Sounds/UI/Camera_Shutter.Camera_Shutter" 1.0 1.0 0.0 0 0)
  (bind _returnvalue (UserInterface|CreateWidget "/Game/Widgets/WB_RoomChange.WB_RoomChange_C"))
  (UserInterface|Viewport|AddtoViewport _returnvalue 0)
  (Default|FadeEvent _returnvalue)
  (Utilities|FlowControl|Delay 1.0)
  (if (== _output_get 1e+01)
    (Game|OpenLevel(byName) "Boss")
    (else
      (bind _newparam (CallFunction|SalaRandom :!label _label))
      (while (== (Math|Conversions|ToInteger(Byte) _newparam) (Variables|/Game/Player/BP_Axololt.BP_Axololt_C|GetRoomNumber _asbp_axololt))
        (Development|PrintString "Repetido")
        (goto _label))
      (Development|PrintString (Utilities|String|ToString(Integer) (Math|Conversions|ToInteger(Byte) _newparam))))))

(event EventBeginPlay
  (bind _asbp_axololt (Utilities|Casting|CastToBP_Axololt (Game|GetPlayerCharacter 0)))
  (Variables|Default|Set%20BP%20Axololt _asbp_axololt))

(fn ConstructionScript)

(fn SalaRandom
  (return (Math|Conversions|ToByte(Integer) (Math|Random|RandomIntegerinRange 0 4))))