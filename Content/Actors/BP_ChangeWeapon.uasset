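; BP_ChangeWeapon is an interactable actor that switches the player's BP_Axololt character between the Ranged and Light weapon types.
; Its Interactable event casts the player character, prints a debug string, then toggles EnumWeapons and the matching WeaponSelected value, followed by a short delay with nothing after it.
; The Box overlap events are unfinished stubs marked TODO and have no effect.
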(event OnComponentBeginOverlap(Box)
  (params (OverlappedComponent :type Primitive%20Component%20Object%20Reference) (OtherActor :type Actor%20Object%20Reference) (OtherComp :type Primitive%20Component%20Object%20Reference) (OtherBodyIndex :type Integer) (bFromSweep :type Boolean) (SweepResult :type Hit%20Result%20Structure%20%28by%20ref%29))
  ;[1 1 1] TODO
  (if (== OtherActor "/Game/Player/BP_Axololt.BP_Axololt")
    _))

(event OnComponentEndOverlap(Box)
  (params (OverlappedComponent :type Primitive%20Component%20Object%20Reference) (OtherActor :type Actor%20Object%20Reference) (OtherComp :type Primitive%20Component%20Object%20Reference) (OtherBodyIndex :type Integer))
  ;[1 1 1] TODO
)

(event EventBeginPlay)

(event Collision|EventActorBeginOverlap
  (params (OtherActor :type Actor%20Object%20Reference)))

(event EventTick
  (params (DeltaSeconds :type Float%20%28single-precision%29)))

(event EventInteractable
  (bind _asbp_axololt (Utilities|Casting|CastToBP_Axololt (Game|GetPlayerCharacter 0)))
  (Development|PrintString "Se Castea")
  (switch Utilities|FlowControl|Switch|SwitchonEnum_Weapons (Variables|/Game/Player/BP_Axololt.BP_Axololt_C|GetEnum_weapons _asbp_axololt)
    (:NewEnumerator0
      (Variables|/Game/Player/BP_Axololt.BP_Axololt_C|SetEnum_weapons _asbp_axololt "NewEnumerator1")
      (Variables|/Game/Player/BP_Axololt.BP_Axololt_C|SetWeaponSelected _asbp_axololt 1.0)
      (Utilities|FlowControl|Delay 0.2))
    (:NewEnumerator1
      (Variables|/Game/Player/BP_Axololt.BP_Axololt_C|SetEnum_weapons _asbp_axololt "NewEnumerator0")
      (Variables|/Game/Player/BP_Axololt.BP_Axololt_C|SetWeaponSelected _asbp_axololt 0.0)
      (Utilities|FlowControl|Delay 0.2))))

(fn ConstructionScript)