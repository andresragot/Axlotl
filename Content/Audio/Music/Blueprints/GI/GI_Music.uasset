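; Game Instance Blueprint that starts the game's battle and merchant music as 2D sounds.
; The battle event spawns its track to persist across level transitions, using a validity check and a playing flag to avoid duplicates.
; The merchant event spawns non-persistent store music only when no valid battle music component exists, and otherwise does nothing.
; Nothing in this graph stops either track or clears the battle flag.
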(event Custom|Spawn_battleMusic
  (Utilities|IsValid (Variables|Default|GetBattle_Music)
    (:Is%20Valid
      (if (not (Variables|Default|GetisPlayingBattle))
        (bind _returnvalue (Audio|SpawnSound2D "/Game/Audio/Music/Samples/SW_Battle.SW_Battle" 0.3 1.0 0.0 0 true))
        (Variables|Default|SetBattle_Music _returnvalue)
        (Variables|Default|SetisPlayingBattle true)))
    (:Is%20Not%20Valid
      (bind _returnvalue_2 (Audio|SpawnSound2D "/Game/Audio/Music/Samples/SW_Battle.SW_Battle" 0.3 1.0 0.0 0 true))
      (Variables|Default|SetBattle_Music _returnvalue_2)
      (Variables|Default|SetisPlayingBattle true))))

(event Custom|SetNewMusicMerchant
  (Utilities|IsValid (Variables|Default|GetBattle_Music)
    (:Is%20Valid
      (if (Variables|Default|GetisPlayingBattle)
        _))
    (:Is%20Not%20Valid
      (bind _returnvalue (Audio|SpawnSound2D "/Game/Audio/Music/Samples/SW_Store.SW_Store" 1.0 1.0 0.0 0))
      (Variables|Default|SetMerchant_Music _returnvalue))))